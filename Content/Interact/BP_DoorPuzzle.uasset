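; BP_DoorPuzzle is a gate that opens once enough fuzes are collected.
; CollectItems reveals a WBP_FuzeOBJ widget and updates its count, then on reaching the maximum removes it and calls OpenDoor once.
; OpenDoor plays the gate level sequence and sound, destroys the actor after a delay, then completes the GateFuze-tagged objective point if it is in progress.
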(event `self.ReceiveBeginPlay`
  (`parent.ReceiveBeginPlay`)
  (bind _returnvalue (`|CreateWidget` "/Game/Quest/WBP_FuzeOBJ.WBP_FuzeOBJ_C"))
  (set `self.NewVar_0` _returnvalue)
  (`UserWidget.AddToViewport` _returnvalue 0)
  (`Widget.SetVisibility` _returnvalue "Hidden"))

(event `OpenDoor`
  (bind (_outactor _returnvalue) (`LevelSequencePlayer.CreateLevelSequencePlayer` "/Game/OpenGateSEQ.OpenGateSEQ"))
  (`MovieSceneSequencePlayer.Play` _returnvalue)
  (`GameplayStatics.PlaySoundAtLocation` "/Game/Sounds/SA_OpenGate.SA_OpenGate" (`self.K2_GetActorLocation`) (struct) 1.0 1.0 0.0 "/Game/Sounds/SA_Gate.SA_Gate" null null null)
  (`KismetSystemLibrary.Delay` 9.0)
  (`self.K2_DestroyActor`)
  (`/Engine/EditorBlueprintResources/StandardMacros.DoOnce` false
    (:`Completed`
      (bind _outactors (`GameplayStatics.GetAllActorsOfClassWithTag` "/Game/ThirdPerson/Blueprints/BP_ObjectivePoints.BP_ObjectivePoints_C" "GateFuze"))
      (bind _output (`|GetArrayItem` _outactors))
      (if (`/Game/ThirdPerson/Blueprints/BP_ObjectivePoints.OBJinProgress?` _output)
        (`/Game/ThirdPerson/Blueprints/BP_ObjectivePoints.CompletedOBJ` _output)))))

(event `CollectItems`
  (bind _newvar_0 (`self.NewVar_0`))
  (`Widget.SetVisibility` _newvar_0 "Visible")
  (bind _result (`/Engine/EditorBlueprintResources/StandardMacros.IncrementInt` (`self.CurrentCollectedItems`))
    (:`  `
      (`TextBlock.SetText` (`/Game/Quest/WBP_FuzeOBJ.CurrentFuze` _newvar_0) (`KismetTextLibrary.Conv_IntToText` _result))
      (if (>= (`self.CurrentCollectedItems`) (`self.MaxItemCollectible`))
        (`/Engine/EditorBlueprintResources/StandardMacros.DoOnce` false
          (:`Completed`
            (`Widget.RemoveFromParent` _newvar_0)
            (`self.OpenDoor`)))))))

(fn `UserConstructionScript`
  (`parent.UserConstructionScript`))