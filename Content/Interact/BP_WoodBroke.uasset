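; BP_WoodBroke is an interactable wood actor that breaks when the E key is pressed.
; The key event destroys the actor, then plays a log-breaking sound at its location with 3D attenuation.
; The graph has no proximity check and does not enable input itself; BeginPlay, overlap and Tick are disabled stubs.
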(event `Key|E`
  (params (Key :type "Key Structure"))
  (:`Pressed`
    (`self.K2_DestroyActor`)
    (`GameplayStatics.PlaySoundAtLocation` "/Game/Sounds/SA_BreakLog.SA_BreakLog" (`self.K2_GetActorLocation`) (struct) 1.0 1.0 0.0 "/Game/Sounds/SA_Audio3d.SA_Audio3d" null null null)))

(fn `UserConstructionScript`
  (`parent.UserConstructionScript`))