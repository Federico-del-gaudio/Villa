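; BP_NumberDoor is a code-locked door that disappears when given the correct code and can complete an objective.
; Pressing E opens WBP_Blueprint with a reference to the door and switches to UI-only input with a visible cursor.
; OpenDoorWithCode checks the code against KeyCode and returns the result.
; A match triggers OpenDoor, which destroys the actor, plays a sound and completes the "DoorNumber"-tagged BP_ObjectivePoints if in progress.
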(event `OpenDoor`
  (`self.K2_DestroyActor`)
  (`GameplayStatics.PlaySoundAtLocation` "/Game/Sounds/SA_Dooeopen.SA_Dooeopen" (`self.K2_GetActorLocation`) (struct) 1.0 1.0 0.0 "/Game/Sounds/SA_Audio3d.SA_Audio3d" null null null)
  (`/Engine/EditorBlueprintResources/StandardMacros.DoOnce` false
    (:`Completed`
      (bind _outactors (`GameplayStatics.GetAllActorsOfClassWithTag` "/Game/ThirdPerson/Blueprints/BP_ObjectivePoints.BP_ObjectivePoints_C" "DoorNumber"))
      (bind _output (`|GetArrayItem` _outactors))
      (if (`/Game/ThirdPerson/Blueprints/BP_ObjectivePoints.OBJinProgress?` _output)
        (`/Game/ThirdPerson/Blueprints/BP_ObjectivePoints.CompletedOBJ` _output)))))

(event `Key|E`
  (params (Key :type "Key Structure"))
  (bind _returnvalue (`GameplayStatics.GetPlayerController` 0))
  (:`Pressed`
    (bind _returnvalue_2 (`|CreateWidget` "/Game/Interact/WBP_Blueprint.WBP_Blueprint_C"))
    (`UserWidget.AddToViewport` _returnvalue_2 0)
    (set `/Game/Interact/WBP_Blueprint.BP_Door` self _returnvalue_2)
    (`WidgetBlueprintLibrary.SetInputMode_UIOnlyEx` _returnvalue null)
    (set `PlayerController.bShowMouseCursor` true _returnvalue)))

(fn `OpenDoorWithCode`
  (params (Code :type String))
  (returns (CorrectCode :type Boolean))
  (if (`KismetStringLibrary.EqualEqual_StrStr` Code (`self.KeyCode`))
    (`self.OpenDoor`)
    (return true)
    (else
      (return false))))

(fn `UserConstructionScript`
  (`parent.UserConstructionScript`))