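; BP_Door is a locked door that the player opens with a key.
; A sphere overlap caches the BP_ThirdPersonCharacter, and no end-overlap handler clears that reference.
; Pressing E checks the cached character's HasKey: if true, the door destroys itself, consumes the key and plays an opening sound.
; Otherwise it plays a locked sound, with both sounds spatialized at the door's location.
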(event `Key|E`
  (params (Key :type "Key Structure"))
  (bind _returnvalue (`self.K2_GetActorLocation`))
  (:`Pressed`
    (if (`/Game/ThirdPerson/Blueprints/BP_ThirdPersonCharacter.HasKey` (stale `self.Sphere.OnComponentBeginOverlap` _asbp_third_person_character))
      (`self.K2_DestroyActor`)
      (set `/Game/ThirdPerson/Blueprints/BP_ThirdPersonCharacter.HasKey` false (stale `self.Sphere.OnComponentBeginOverlap` _asbp_third_person_character))
      (`GameplayStatics.PlaySoundAtLocation` "/Game/Sounds/SA_Dooeopen.SA_Dooeopen" _returnvalue (struct) 1.0 1.0 0.0 "/Game/Sounds/SA_Audio3d.SA_Audio3d" null null null)
      (else
        (`GameplayStatics.PlaySoundAtLocation` "/Game/Sounds/SA_KeyLock.SA_KeyLock" _returnvalue (struct) 1.0 1.0 0.0 "/Game/Sounds/SA_Audio3d.SA_Audio3d" null null null)))))

(event `self.Sphere.OnComponentBeginOverlap`
  (params (OverlappedComponent :type "PrimitiveComponent Object Reference") (OtherActor :type "Actor Object Reference") (OtherComp :type "PrimitiveComponent Object Reference") (OtherBodyIndex :type Integer) (bFromSweep :type Boolean) (SweepResult :type "HitResult Structure (by ref)"))
  (bind _asbp_third_person_character (cast `/Game/ThirdPerson/Blueprints/BP_ThirdPersonCharacter` OtherActor)))

(fn `UserConstructionScript`
  (`parent.UserConstructionScript`))