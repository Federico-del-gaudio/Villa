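; BP_AI is an AI pawn that patrols and investigates noises.
; On BeginPlay it sets walk speed from MaxWalkSpeed and moves to a random reachable point within Radius of itself, repeating on each success.
; When PawnSensing hears a noise, it moves to that location and prints debug strings.
; Neither a failed patrol move nor a finished investigation restarts the patrol.
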(event `self.ReceiveBeginPlay`
  (`self.AIMovePatroll`))

(event `AIMovePatroll`
  (set `CharacterMovementComponent.MaxWalkSpeed` (`self.Max Walk Speed`) (`self.CharacterMovement`))
  (`|AIMoveTo` self (`NavigationSystemV1.K2_GetRandomReachablePointInRadius` (`self.K2_GetActorLocation`) (`self.Radius`) null null) null
    (:`OnSuccess`
      (`self.AIMovePatroll`))))

(event `self.PawnSensing.OnHearNoise`
  (params (Instigator :type "Pawn Object Reference") (Location :type "Vector Structure (by ref)") (Volume :type "Float (single-precision)"))
  (`KismetSystemLibrary.PrintString` "Hello")
  (`|AIMoveTo` self Location null
    (:`OnSuccess`
      (`KismetSystemLibrary.PrintString` "success"))
    (:`OnFail`
      (`KismetSystemLibrary.PrintString` "Fail"))))

(fn `UserConstructionScript`)