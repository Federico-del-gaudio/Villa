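; Enemy AI character that patrols random reachable points, investigates noises and hunts the player by sound.
; Separate hearing events speed it up toward either a non-player noise location or the player's position, with randomized timers after moves.
; DoOnce gates control chase music, using a GameMode flag to avoid overlapping object-chase tracks.
; Reaching the player enables a jumpscare collision whose overlap triggers the character's death sequence and stops player-chase music.
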(event `PlayScreamPatrol`
  (`GameplayStatics.SpawnSoundAttached` "/Game/Sounds/Enemy/SA_ScreamPatrol.SA_ScreamPatrol" (`self.Mesh`) "None" (0.0 0.0 0.0) (struct) "KeepRelativeOffset" false 0.85 1.0 0.0 "/Game/Sounds/Enemy/SA_Patrol.SA_Patrol" null))

(event `self.ReceiveBeginPlay`
  ; Patrol
  (`self.AIMovePatroll`)
  (set `self.PlayerKilled?` false)
  (bind _asbp_third_person_game_mode (cast `/Game/ThirdPerson/Blueprints/BP_ThirdPersonGameMode` (`GameplayStatics.GetGameMode`)))
  (set `self.As BP Third Person Game Mode` _asbp_third_person_game_mode))

(event `AIMovePatroll`
  (bind _as_bp_third_person_game_mode (`self.As BP Third Person Game Mode`))
  (bind _ismusicplaying (`/Game/ThirdPerson/Blueprints/BP_ThirdPersonGameMode.IsMusicPlaying` _as_bp_third_person_game_mode))
  ; Patrol
  (`KismetSystemLibrary.K2_SetTimerDelegate` (`|CreateDelegate` :!event `PlayScreamPatrol`) (`KismetMathLibrary.RandomFloatInRange` 3.0 18.0))
  (set `CharacterMovementComponent.MaxWalkSpeed` (`self.Max Walk Speed`) (`self.CharacterMovement`))
  (`|AIMoveTo` self (`NavigationSystemV1.K2_GetRandomReachablePointInRadius` (`self.K2_GetActorLocation`) (`self.Radius`) null null) null 100.0
    (:`then`
      ; Patrol to noise (no player)
      (`|ExecutionSequence`
        (:`then_0`
          (goto _label_2 :!via `Reset`))
        (:`then_1`
          (`/Engine/EditorBlueprintResources/StandardMacros.DoOnce` false :!label _label
            (:`Completed`
              (bind _musicchase (`self.MusicChase`)
                (:`then`
                  (`AudioComponent.FadeOut` _musicchase 0.5 0.0 "Linear")
                  (set `/Game/ThirdPerson/Blueprints/BP_ThirdPersonGameMode.IsMusicPlaying` false (`self.As BP Third Person Game Mode`)))
                (:`else`)))))))
    (:`OnSuccess`
      (`KismetSystemLibrary.K2_SetTimerDelegate` (`|CreateDelegate` :!event `AIMovePatroll`) (`KismetMathLibrary.RandomFloatInRange` 2.0 8.0)))))

(event `self.HearObject.OnHearNoise`
  (params (Instigator :type "Pawn Object Reference") (Location :type "Vector Structure (by ref)") (Volume :type "Float (single-precision)"))
  (bind _as_bp_third_person_game_mode (`self.As BP Third Person Game Mode`))
  (bind _ismusicplaying (`/Game/ThirdPerson/Blueprints/BP_ThirdPersonGameMode.IsMusicPlaying` _as_bp_third_person_game_mode))
  ; Patrol to noise (no player)
  (if (not (`self.ActorHasTag` Instigator "Player"))
    (set `self.Sound location` (`self.K2_GetActorLocation` Instigator))
    (set `CharacterMovementComponent.MaxWalkSpeed` 850.0 (`self.CharacterMovement`))
    (`self.Move to object`)
    (`|ExecutionSequence`
      (:`then_0`
        (`/Engine/EditorBlueprintResources/StandardMacros.DoOnce` _ismusicplaying :!label _label_2
          (:`Completed`
            ; Patrol
            (if (not _ismusicplaying)
              (set `/Game/ThirdPerson/Blueprints/BP_ThirdPersonGameMode.IsMusicPlaying` true _as_bp_third_person_game_mode)
              (bind _returnvalue (`GameplayStatics.SpawnSoundAttached` "/Game/Sounds/Enemy/SA_ChaseOBJ.SA_ChaseOBJ" (`self.Mesh`) "None" (0.0 0.0 0.0) (struct) "KeepRelativeOffset" false 1.0 1.0 0.0 "/Game/Sounds/SA_Chaseobb.SA_Chaseobb" null))
              (set `self.MusicChase` _returnvalue)))))
      (:`then_1`
        (goto _label :!via `Reset`)))))

(event `Move to object`
  ; Patrol to noise (no player)
  (bind _returnvalue (`NavigationSystemV1.FindPathToLocationSynchronously` (`self.K2_GetActorLocation`) (`self.Sound location`) null null))
  (if (`KismetSystemLibrary.IsValid` _returnvalue)
    (if (not (`NavigationPath.IsPartial` _returnvalue))
      (`|AIMoveTo` self (`self.Sound location`) null 350.0
        (:`OnSuccess`
          (`KismetSystemLibrary.K2_SetTimerDelegate` (`|CreateDelegate` :!event `AIMovePatroll`) (`KismetMathLibrary.RandomFloatInRange` 2.0 9.0)))))
    (else
      (`self.AIMovePatroll`))))

(event `self.HearPlayer.OnHearNoise`
  (params (Instigator :type "Pawn Object Reference") (Location :type "Vector Structure (by ref)") (Volume :type "Float (single-precision)"))
  (`KismetSystemLibrary.PrintString` "Ti sento")
  (`self.Move to player`)
  (`/Engine/EditorBlueprintResources/StandardMacros.DoOnce` false :!label _label_3
    (:`Completed`
      ; Chase player
      (`AudioComponent.Play` (`self.Chae`) 0.0)
      (set `self.MusicPaying` true))))

(event `Move to player`
  ; Chase player
  (set `CharacterMovementComponent.MaxWalkSpeed` 780.0 (`self.CharacterMovement`))
  (`|AIMoveTo` self (`self.K2_GetActorLocation` (`GameplayStatics.GetPlayerCharacter` 0)) null 1.0
    (:`OnSuccess`
      (`PrimitiveComponent.SetCollisionEnabled` (`self.JumpscareCollision`) "QueryOnly")
      (if (`self.PlayerKilled?`)
        (`PrimitiveComponent.SetCollisionEnabled` (`self.JumpscareCollision`) "NoCollision")
        (`KismetSystemLibrary.K2_SetTimerDelegate` (`|CreateDelegate` :!event `AIMovePatroll`) (`KismetMathLibrary.RandomFloatInRange` 2.0 5.0))
        (else
          (`KismetSystemLibrary.K2_SetTimerDelegate` (`|CreateDelegate` :!event `AIMovePatroll`) (`KismetMathLibrary.RandomFloatInRange` 2.0 5.0)))))))

(event `self.JumpscareCollision.OnComponentBeginOverlap`
  (params (OverlappedComponent :type "PrimitiveComponent Object Reference") (OtherActor :type "Actor Object Reference") (OtherComp :type "PrimitiveComponent Object Reference") (OtherBodyIndex :type Integer) (bFromSweep :type Boolean) (SweepResult :type "HitResult Structure (by ref)"))
  (bind _asbp_third_person_character (cast `/Game/ThirdPerson/Blueprints/BP_ThirdPersonCharacter` OtherActor))
  (`/Game/ThirdPerson/Blueprints/BP_ThirdPersonCharacter.DeathSequence` _asbp_third_person_character)
  (set `self.PlayerKilled?` true)
  (if (`self.MusicPaying`)
    (`AudioComponent.Stop` (`self.Chae`))
    (set `self.MusicPaying` false)
    (goto _label_3 :!via `Reset`)))

(fn `UserConstructionScript`)